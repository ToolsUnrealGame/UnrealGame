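; BP_SpringBoard is a platform actor that sinks a short distance while anything overlaps its Box and rises back when the box is empty.
; Each Tick picks the lowered or initial location as the target and eases toward it with a delta-time-scaled lerp, without sweeping.
; The same overlap check drives the TransferCollision component's TransferCollisionToPlatform flag.
; No launch or bounce impulse is applied here.
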(event `self.ReceiveBeginPlay`
  (bind _returnvalue (`self.K2_GetActorLocation`))
  (set `self.Distance` 15.0)
  (set `self.InitialLocation` _returnvalue)
  (set `self.TargetLocation` _returnvalue))

(event `self.ReceiveTick`
  (params (DeltaSeconds :type "Float (single-precision)"))
  (bind _transfercollision (`self.TransferCollision`))
  (if (>= (`KismetArrayLibrary.Array_Length` (`PrimitiveComponent.GetOverlappingActors` (`self.Box`) null)) 1)
    (set `self.TargetLocation` (+ (* (`self.Distance`) (`KismetMathLibrary.Vector_Down`)) (`self.InitialLocation`)))
    (`TransferCollision.TransferCollisionToPlatform` _transfercollision true)
    (else
      (set `self.TargetLocation` (`self.InitialLocation`))
      (`TransferCollision.TransferCollisionToPlatform` _transfercollision false)))
  (`self.K2_SetActorLocation` (`KismetMathLibrary.VLerp` (`self.K2_GetActorLocation`) (`self.TargetLocation`) (* DeltaSeconds 5.0))))

(fn `UserConstructionScript`)